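; Player controller for the WoE login stage that keeps the Photon networking service pumped.
; On BeginPlay it starts a looping half-second timer that calls PhotonCallService on the WoEGameInstance and prints a debug message on each successful call.
; A status-change handler prints an on-screen notice when the server connection reports Disconnected.
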(event EventBeginPlay
  (Utilities|Time|SetTimerbyFunctionName 0 "CallPhotonService" 0.5 true))

(event EventTick
  (params (DeltaSeconds :type Float%20%28single-precision%29)))

(event EventHandleStatusChanged
  (params (FStatusCode :type Integer))
  (if (== FStatusCode (Variables|Default|GetDisconnected))
    (Development|PrintString "Just Disconnected from the Server!" true true "(R=0.000000,G=0.660000,B=1.000000,A=1.000000)" 1e+01)))

(fn ConstructionScript)

(fn CallPhotonService
  (bind _aswo_egame_instance (Utilities|Casting|CastToWoEGameInstance (Game|GetGameInstance)))
  (Class|WoEGameInstance|PhotonCallService _aswo_egame_instance true)
  (Development|PrintString "Called by timer." true true "(R=0.000000,G=1.000000,B=0.044180,A=1.000000)" 1.0))